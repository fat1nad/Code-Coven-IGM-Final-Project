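; BP_SpinningDoppleganger is an actor that travels along the spline of the level's BP_SpinningSpline actor.
; On BeginPlay it finds that spline, then waits MyDelay so each doppelganger can launch at a staggered time.
; Move plays a timeline at a rate of 1/TimeToComplete, mapping its track to spline distance.
; Each update sets the actor's location in world space and its rotation from the spline's local space.
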(event Custom|Move
  (bind _spinning_spline (Variables|Default|GetSpinning%20Spline))
  (bind _spline (Variables|/Game/BluePrints/BP_SpinningSpline.BP_SpinningSpline_C|GetSpline _spinning_spline))
  (Components|Timeline|SetPlayRate (Variables|Default|GetMove%20Timeline) (/ 1.0 (Variables|Default|GetTime%20To%20Complete)))
  (bind _move_track (Timeline|Move%20Timeline Play)
    (:Update
      (Transformation|SetActorTransform (Math|Transform|MakeTransform (Spline|GetLocationatDistanceAlongSpline _spline (Math|Float|Lerp 0.0 (Spline|GetSplineLength (Variables|/Game/BluePrints/BP_SpinningSpline.BP_SpinningSpline_C|GetSpline (Variables|Default|GetSpinning%20Spline))) _move_track) "World") (Spline|GetRotationatDistanceAlongSpline _spline (Math|Float|Lerp 0.0 (Spline|GetSplineLength (Variables|/Game/BluePrints/BP_SpinningSpline.BP_SpinningSpline_C|GetSpline (Variables|Default|GetSpinning%20Spline))) _move_track) "Local") "1,1,1")))))

(event EventBeginPlay
  ;[1 1 1] When play starts, get a reference to the spline
  (bind _returnvalue (Actor|GetActorOfClass "/Game/BluePrints/BP_SpinningSpline.BP_SpinningSpline_C"))
  (Variables|Default|SetSpinning%20Spline _returnvalue)
  ;[1 1 1] Add a delay to each doppel before launching it
  (Utilities|FlowControl|Delay (Variables|Default|GetMyDelay))
  (CallFunction|Move))

(fn ConstructionScript)