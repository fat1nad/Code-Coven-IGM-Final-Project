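; BP_Doppleganger is a double that shadows the ThirdPersonCharacter, referenced as Megan, by copying its movement at a fixed offset.
; BeginPlay finds the character and stores the vector from itself to Megan.
; Tick adds that vector to Megan's location without sweeping, so it sits opposite its placed side of her.
; Only location follows; rotation and animation are not copied.
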(event EventBeginPlay
  (bind _returnvalue (Actor|GetActorOfClass "/Game/ThirdPersonBP/Blueprints/ThirdPersonCharacter.ThirdPersonCharacter_C"))
  (bind _output_get (Variables|Default|SetMegan _returnvalue))
  (Variables|Default|SetOffsetFromMegan (- (Transformation|GetActorLocation _output_get) (Transformation|GetActorLocation))))

(event EventTick
  (params (DeltaSeconds :type Float%20%28single-precision%29))
  (Transformation|SetActorLocation (+ (Transformation|GetActorLocation (Variables|Default|GetMegan)) (Variables|Default|GetOffsetFromMegan)) false false))

(fn ConstructionScript)