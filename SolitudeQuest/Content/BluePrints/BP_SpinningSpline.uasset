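; BP_SpinningSpline is a spline actor that follows the player character, Megan, at a fixed offset.
; On BeginPlay it finds the ThirdPersonCharacter and stores its own starting X and Y offset from her, with a constant Z offset.
; Every Tick it moves itself to her location plus that offset without sweeping.
; The graphs only translate the actor; no spinning logic appears here.
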(event EventBeginPlay
  ;[1 1 1] When play starts, get a reference to real Megan
  (bind _returnvalue (Actor|GetActorOfClass "/Game/ThirdPersonBP/Blueprints/ThirdPersonCharacter.ThirdPersonCharacter_C"))
  (bind _output_get (Variables|Default|SetMeganPlayer _returnvalue))
  (Variables|Default|SetOffsetFromMegan (Math|Vector|MakeVector (.X (Math|Vector|BreakVector (- (Transformation|GetActorLocation) (Transformation|GetActorLocation _output_get)))) (.Y (Math|Vector|BreakVector (- (Transformation|GetActorLocation) (Transformation|GetActorLocation _output_get)))) 1e+01)))

(event EventTick
  (params (DeltaSeconds :type Float%20%28single-precision%29))
  ;[1 1 1] On each frame, offset the spline from real Megan
  (Transformation|SetActorLocation (+ (Transformation|GetActorLocation (Variables|Default|GetMeganPlayer)) (Variables|Default|GetOffsetFromMegan)) false false))

(fn ConstructionScript)